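; Camera rail actor that takes over the player's view and positions itself along a rail based on trigger boxes.
; When the main character enters its blend volume, the player controller blends to the first rail of this class found in the level, rather than explicitly to itself.
; BoxTriggered maps the trigger's index in the box array to a normalized 0–1 rail position.
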(event `self.CameraBlendVolume.OnComponentBeginOverlap`
  (params (OverlappedComponent :type "PrimitiveComponent Object Reference") (OtherActor :type "Actor Object Reference") (OtherComp :type "PrimitiveComponent Object Reference") (OtherBodyIndex :type Integer) (bFromSweep :type Boolean) (SweepResult :type "HitResult Structure (by ref)"))
  (bind _asbeu_main_character_bp (cast `/Game/OurGameFolder/BEU_Blueprints/BEU_MainCharacter_BP` OtherActor))
  (bind _asplayer_controller (cast `PlayerController` (`Pawn.GetController` _asbeu_main_character_bp)))
  (bind _returnvalue (`GameplayStatics.GetActorOfClass` "BEU_CameraRail_BP_C"))
  (`PlayerController.SetViewTargetWithBlend` _asplayer_controller _returnvalue (`self.CameraBlendTime`) "VTBlend_Linear" 0.0 false))

(event `/Game/OurGameFolder/BEU_Blueprints/Interfaces/BEU_TriggerBox_IF.BoxTriggered`
  (params (Trigger :type "Actor Object Reference"))
  (for (_array_element _array_index) (`self.TriggerBoxArray`)
    (if (== Trigger _array_element)
      (break)))
  (set `self.CurrentPositionOnRail` (`KismetMathLibrary.MapRangeClamped` (`KismetMathLibrary.Conv_IntToDouble` _array_index) 0.0 (- (`KismetMathLibrary.Conv_IntToDouble` (`KismetArrayLibrary.Array_Length` (`self.TriggerBoxArray`))) 1.0) 0.0 1.0)))

(fn `UserConstructionScript`)