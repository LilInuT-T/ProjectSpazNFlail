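; Player character Blueprint for a flipbook-sprite beat 'em up, with movement, jumping, light and heavy attacks, health and death.
; The Construction Script fills the flipbook set from a character enum (Water Spirit or Tree Hugger), with some slots empty.
; Custom events take movement and attack input, while Tick picks the flipbook by state and ends attacks on the last frame.
; Combos are only flagged, DoDamageCE is empty, and B applies test damage.
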(event `DeathCE`
  (bind _characterfb (`self.CharacterFB`))
  ;[1 1 1] Death Event- flipbook change and TBD action
  (`PaperFlipbookComponent.SetFlipbook` _characterfb (`self.DeathFB`))
  (if (>= (`PaperFlipbookComponent.GetPlaybackPositionInFrames` _characterfb) (- (`PaperFlipbookComponent.GetFlipbookLengthInFrames` _characterfb) 1))
    (`PaperFlipbookComponent.Stop` _characterfb)
    (`KismetSystemLibrary.Delay` 5.0)))

(event `AttackCE`
  (bind _characterfb (`self.CharacterFB`))
  (bind _returnvalue (>= (`PaperFlipbookComponent.GetPlaybackPositionInFrames` _characterfb) (- (`PaperFlipbookComponent.GetFlipbookLengthInFrames` _characterfb) 1)))
  ;[1 1 1] Attack Event- character attacks
  (if (not (`self.ComboInput?`))
    (switch `/Game/OurGameFolder/BEU_Blueprints/ENUMs/BEU_Attack_ENUM` (`self.AttackInputENUM`)
      (:`NewEnumerator0`
        (`PaperFlipbookComponent.SetFlipbook` _characterfb (`self.LightAttackFB`))
        (if _returnvalue
          (set `self.IsAttacking` false :!label _label)))
      (:`NewEnumerator1`
        (`PaperFlipbookComponent.SetFlipbook` _characterfb (`self.HeavyAttackFB`))
        (if _returnvalue
          (goto _label))))))

(event `self.ReceiveTick`
  (params (DeltaSeconds :type "Float (single-precision)"))
  (bind (_returnvalue_x _returnvalue_y _returnvalue_z) (`KismetMathLibrary.BreakVector` (`self.GetVelocity`)))
  (`|ExecutionSequence`
    (:`then_0`
      (if (`self.IsDead`)
        (`self.DeathCE`)
        (elif (`self.IsAttacking`)
          (`self.AttackCE`)
          (else
            (bind _output_get (set `self.MovingUp` (!= _returnvalue_z 0.0)))
            (if _output_get
              (`PaperFlipbookComponent.SetFlipbook` (`self.CharacterFB`) (`self.JumpFB`))
              (else
                (bind _output_get_2 (set `self.MovingRight` (!= _returnvalue_x 0.0)))
                (bind _output_get_3 (set `self.MovingForward` (!= _returnvalue_y 0.0)))
                (if (or _output_get_3 _output_get_2)
                  (`PaperFlipbookComponent.SetFlipbook` (`self.CharacterFB`) (`self.WalkFB`))
                  (else
                    (`PaperFlipbookComponent.SetFlipbook` (`self.CharacterFB`) (`self.IdleFB`))))))))))))

(event `TakeDamageCE`
  (params (DamageDealt :type "Float (double-precision)"))
  ;[1 1 1] Take Damage Event- Damage is subtracted from health
  (bind _output_get (set `self.CurrentHealth` (- (`self.CurrentHealth`) DamageDealt)))
  (set `self.IsDead` (<= _output_get 0.0)))

(event `AttackInputRecievedCE`
  (params (AttackInput :type "/Game/OurGameFolder/BEU_Blueprints/ENUMs/BEU_Attack_ENUM Enum" :default "NewEnumerator0"))
  ;[1 1 1] Attack Input Event- attack input from controller is received
  (set `self.AttackInputENUM` AttackInput)
  (if (`self.IsDead`)
    _
    (elif (`self.IsAttacking`)
      (set `self.ComboInput?` true)
      (else
        (set `self.IsAttacking` true)))))

(event `Key|B`
  (params (Key :type "Key Structure"))
  ;[1 1 0] Test button
  (:`Pressed`
    (`self.TakeDamageCE` 0.25)))

(event `JumpCE`
  ;[1 1 1] Jump Event- character jumps
  (if (not (or (`self.IsDead`) (`self.IsAttacking`)))
    (`self.Jump`)))

(event `DoDamageCE`)

(event `WalkRight/LeftCE`
  (params (AxisValue :type "Float (double-precision)"))
  ;[1 1 1] Walk Left/Right Event- moves character and changes sprite facing
  (if (not (or (`self.IsDead`) (`self.IsAttacking`)))
    (`self.AddMovementInput` (`KismetMathLibrary.Vector_Right`) AxisValue)
    (if (> AxisValue 0.0)
      (`SceneComponent.K2_SetRelativeRotation` :`self` (`self.CharacterFB`))
      (elif (< AxisValue 0.0)
        (`SceneComponent.K2_SetRelativeRotation` (`self.CharacterFB`) (struct :`Yaw` 180.0) false false)))))

(event `WalkIn/OutCE`
  (params (AxisValue :type "Float (single-precision)"))
  ;[1 1 1] Walk In/Out Event- moves character
  (if (not (or (`self.IsDead`) (`self.IsAttacking`)))
    (`self.AddMovementInput` (`KismetMathLibrary.Vector_Forward`) AxisValue)))

(event `self.ReceiveBeginPlay`
  (set `self.ActiveController` (`GameplayStatics.GetPlayerController` 0)))

(fn `UserConstructionScript`
  (bind _characterfb (`self.CharacterFB`))
  (switch `/Game/OurGameFolder/BEU_Blueprints/ENUMs/BEU_Character_ENUM` (`self.Character_ENUM_Select`)
    (:`NewEnumerator0`
      (`PaperFlipbookComponent.SetFlipbook` _characterfb null)
      (set `self.IdleFB` null)
      (set `self.WalkFB` "/Game/OurGameFolder/MySprites/WaterSpirit/BEU_WaterSpirit_Walk_FB.BEU_WaterSpirit_Walk_FB")
      (set `self.JumpFB` null)
      (set `self.LightAttackFB` "/Game/OurGameFolder/MySprites/WaterSpirit/BEU_WaterSpirit_LightAttack_FB.BEU_WaterSpirit_LightAttack_FB")
      (set `self.HeavyAttackFB` "/Game/OurGameFolder/MySprites/WaterSpirit/BEU_WaterSpirit_HeavyAttack_FB.BEU_WaterSpirit_HeavyAttack_FB")
      (set `self.DeathFB` "/Game/OurGameFolder/MySprites/WaterSpirit/BEU_WaterSpirit_Death_FB.BEU_WaterSpirit_Death_FB")
      (set `self.TauntFB` null))
    (:`NewEnumerator1`
      (`PaperFlipbookComponent.SetFlipbook` _characterfb "/Game/OurGameFolder/MySprites/TreeHugger/BEU_TreeHugger1_Idle_FB.BEU_TreeHugger1_Idle_FB")
      (set `self.IdleFB` "/Game/OurGameFolder/MySprites/TreeHugger/BEU_TreeHugger1_Idle_FB.BEU_TreeHugger1_Idle_FB")
      (set `self.WalkFB` "/Game/OurGameFolder/MySprites/TreeHugger/BEU_TreeHugger1_Walk_FB.BEU_TreeHugger1_Walk_FB")
      (set `self.JumpFB` null)
      (set `self.LightAttackFB` "/Game/OurGameFolder/MySprites/TreeHugger/BEU_TreeHugger1_LightAttack_FB.BEU_TreeHugger1_LightAttack_FB")
      (set `self.HeavyAttackFB` null)
      (set `self.DeathFB` null)
      (set `self.TauntFB` null))))