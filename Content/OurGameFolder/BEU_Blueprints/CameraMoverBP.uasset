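; CameraMoverBP is a camera rail volume that guides the player character's camera along a track.
; Player overlap with InfluenceBox toggles tracking on and off.
; While active, Tick interpolates the BEU player's CharacterCamera toward the point on the Track spline closest to the player, using InterpSpeed.
; It moves only the camera's world location, leaving rotation untouched, and does not restore the position on exit.
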(event `self.ReceiveBeginPlay`
  (bind _asbeu_player_character_bp (cast `/Game/OurGameFolder/BEU_Blueprints/BEU_PlayerCharacter_BP` (`GameplayStatics.GetPlayerCharacter` 0)))
  (set `self.PlayerRef` _asbeu_player_character_bp))

(event `self.InfluenceBox.OnComponentBeginOverlap`
  (params (OverlappedComponent :type "PrimitiveComponent Object Reference") (OtherActor :type "Actor Object Reference") (OtherComp :type "PrimitiveComponent Object Reference") (OtherBodyIndex :type Integer) (bFromSweep :type Boolean) (SweepResult :type "HitResult Structure (by ref)"))
  (cast `/Game/OurGameFolder/BEU_Blueprints/BEU_PlayerCharacter_BP` OtherActor)
  (set `self.ActiveTrack` true))

(event `self.InfluenceBox.OnComponentEndOverlap`
  (params (OverlappedComponent :type "PrimitiveComponent Object Reference") (OtherActor :type "Actor Object Reference") (OtherComp :type "PrimitiveComponent Object Reference") (OtherBodyIndex :type Integer))
  (cast `/Game/OurGameFolder/BEU_Blueprints/BEU_PlayerCharacter_BP` OtherActor)
  (set `self.ActiveTrack` false))

(event `self.ReceiveTick`
  (params (DeltaSeconds :type "Float (single-precision)"))
  (bind _charactercamera (`/Game/OurGameFolder/BEU_Blueprints/BEU_MainCharacter_BP.CharacterCamera` (`self.PlayerRef`)))
  (if (`self.ActiveTrack`)
    (set `self.DeltaSec` DeltaSeconds)
    (set `self.CurrentCameraLocation` (`SceneComponent.K2_GetComponentLocation` _charactercamera))
    (`SceneComponent.K2_SetWorldLocation` _charactercamera (`KismetMathLibrary.VInterpTo` (`self.CurrentCameraLocation`) (`SplineComponent.FindLocationClosestToWorldLocation` (`self.Track`) (`self.K2_GetActorLocation` (`self.PlayerRef`)) "World") (`self.DeltaSec`) (`self.InterpSpeed`)) false false)))

(fn `UserConstructionScript`)